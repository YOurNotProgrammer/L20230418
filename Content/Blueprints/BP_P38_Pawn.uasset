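; Player-controlled P-38 plane pawn that flies forward continuously and fires rockets.
; Tick feeds movement input along the actor's forward vector, scaled by Speed and delta time, and spins both propellers through a shared RotatePropeller function.
; Enhanced Input drives frame-rate-scaled local pitch and roll rotation.
; The fire action spawns BP_Rocket at the Arrow component's transform, skipping the spawn if it would collide.
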(event Input|EnhancedActionEvents|EnhancedInputActionIA_PitchRoll
  (params (ActionValue :type Vector%202D%20Structure) (ElapsedSeconds :type Float%20%28double-precision%29) (TriggeredSeconds :type Float%20%28double-precision%29) (InputAction :type Input%20Action%20Object%20Reference :default "/Game/Blueprints/Input/IA_PitchRoll.IA_PitchRoll"))
  (:Triggered
    (Transformation|AddActorLocalRotation (* (Math|Rotator|MakeRotator (.x ActionValue) (.y ActionValue) 0.0) (Utilities|Time|GetWorldDeltaSeconds) 6e+01) false false)))

(event Input|EnhancedActionEvents|EnhancedInputActionIA_Fire
  (params (ActionValue :type Boolean) (ElapsedSeconds :type Float%20%28double-precision%29) (TriggeredSeconds :type Float%20%28double-precision%29) (InputAction :type Input%20Action%20Object%20Reference :default "/Game/Blueprints/Input/IA_Fire.IA_Fire"))
  (bind _self self)
  (:Triggered
    (Game|SpawnActorfromClass "/Game/Blueprints/BP_Rocket.BP_Rocket_C" (Transformation|GetWorldTransform (Variables|Default|GetArrow)) "DontSpawnIfColliding" _self _self)))

(event EventTick
  (params (DeltaSeconds :type Float%20%28single-precision%29))
  (Utilities|FlowControl|Sequence
    (:then_0
      (Pawn|Input|AddMovementInput (Transformation|GetActorForwardVector) (* (Utilities|Time|GetWorldDeltaSeconds) (Variables|Speed|GetSpeed)) false))
    (:then_1
      (CallFunction|RotatePropeller (Variables|Default|GetRight_Propeller)))
    (:then_2
      (CallFunction|RotatePropeller (Variables|Default|GetLeft_Propeller)))))

(fn ConstructionScript)

(fn RotatePropeller
  (params (Where :type Static%20Mesh%20Component%20Object%20Reference))
  (Transformation|AddRelativeRotation Where (Math|Rotator|MakeRotator (* (Utilities|Time|GetWorldDeltaSeconds) (Variables|Speed|GetRotateSpeed)) 0.0 0.0) false false))